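; VHCharacter_BP is a player character that gets visibly marked as detected when damaged or idle, and can launch a scan wave.
; The server runs damage, death and an idle timer that restarts on movement, while detection updates toggle "Painted" on dynamic weapon and mask materials.
; Clients drive the scan through a material parameter collection and handle health UI and respawn, with a Possessed hack covering spawn replication delay.
; Mask and weapon meshes are random or fixed variants.
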(event `self.ReceiveBeginPlay`
  (bind _mask (`self.Mask`))
  (`|ExecutionSequence`
    (:`then_0`
      (`self.UpdateProps`))
    (:`then_1`
      (bind _returnvalue (`KismetMaterialLibrary.CreateDynamicMaterialInstance` "/Game/Materials/Paint_MI.Paint_MI"))
      (bind _output_get (set `self.WeaponMaterial` _returnvalue))
      (`PrimitiveComponent.SetMaterial` (`self.Weapon`) 1 _output_get))
    (:`then_2`
      (bind _returnvalue_2 (`PrimitiveComponent.CreateDynamicMaterialInstance` _mask 0 (`PrimitiveComponent.GetMaterial` _mask 0) "None"))
      (set `self.MaskMaterial` _returnvalue_2))
    (:`then_3`
      (`self.UpdateDetectedState` false))
    (:`then_4`
      (`self.ResetIdle` true))))

(event `self.OnScan`
  ;[1 1 1] [Client] Launch Scan wave
  (`|ExecutionSequence`
    (:`then_1`
      (`KismetMaterialLibrary.SetVectorParameterValue` "/Game/Materials/ScanParameters.ScanParameters" "Location" (`KismetMathLibrary.Conv_VectorToLinearColor` (`self.K2_GetActorLocation`)))
      (`KismetMaterialLibrary.SetScalarParameterValue` "/Game/Materials/ScanParameters.ScanParameters" "LaunchTime" (`GameplayStatics.GetTimeSeconds`))
      (`KismetMaterialLibrary.SetScalarParameterValue` "/Game/Materials/ScanParameters.ScanParameters" "Power" 1.0))
    (:`then_2`
      (`KismetSystemLibrary.RetriggerableDelay` 5.0)
      (`KismetMaterialLibrary.SetScalarParameterValue` "/Game/Materials/ScanParameters.ScanParameters" "Power"))))

(event `self.ReceiveTick`
  (params (DeltaSeconds :type "Float (single-precision)"))
  (bind _returnvalue (`SceneComponent.K2_GetComponentLocation` (`self.FP_MuzzleLocation`)))
  (`|ExecutionSequence`
    (:`then_0`
      ;[1 1 1] Update Look rotation for the animation blueprint
      (bind _output_get (set `self.LookTarget` (* (`KismetMathLibrary.GetForwardVector` (`self.GetBaseAimRotation`)) 5000.0)))
      ;[1 1 1] Debug output
      (if (`self.bDebug`)
        (`KismetSystemLibrary.DrawDebugLine` _returnvalue (+ _returnvalue _output_get) (struct :`G` 1.0 :`B` 0.035417 :`A` 1.0) 0.1 2.0)))
    (:`then_1`
      ;[1 1 1] Reset Idle state on movement
      (`self.ResetIdle` false))))

(event `self.OnDetectionUpdate`
  (`self.UpdateDetectedState` false))

(event `self.OnHealthUpdated`
  ;[1 1 1] [Client] Update health UI for client
  (`self.OnHealthUpdate`))

(event `self.ReceiveAnyDamage`
  (params (Damage :type "Float (single-precision)") (DamageType :type "DamageType Object Reference") (InstigatedBy :type "Controller Object Reference") (DamageCauser :type "Actor Object Reference"))
  ;[1 1 1] [Server] On damage received
  (`|ExecutionSequence`
    (:`then_0`
      (set `self.CurrentHealth` (- (`self.CurrentHealth`) Damage))
      ;;[1 1 1] Update health UI for server
      (`self.OnHealthUpdate`))
    (:`then_1`
      (if (== (`self.CurrentHealth`) 0.0)
        (bind _asvhplayer_controller (cast `/Game/Blueprints/VHPlayerController` (`self.GetController`)))
        (`/Game/Blueprints/VHPlayerController.Death` _asvhplayer_controller)
        (else
          (`self.SetDetected`))))))

(event `self.ReceivePossessed`
  (params (NewController :type "Controller Object Reference"))
  ;[1 0.2783 0] Hack to handle spawn replication delay
  ;;[1 1 1] [Server]
  (`self.OnRespawned`))

(event `OnRespawned`
  ;[1 0.2783 0] Hack to handle spawn replication delay
  ;;[1 1 1] [Client]
  (if (`self.IsLocallyControlled`)
    (bind _asvhplayer_controller (cast `/Game/Blueprints/VHPlayerController` (`self.GetController`)))
    (`/Game/Blueprints/VHPlayerController.OnRespawn` _asvhplayer_controller)))

(fn `DetectedByIdle`
  (`self.ResetIdle` true true)
  (`self.SetDetected`))

(fn `ResetIdle`
  (params (bForced :type Boolean) (bIsIdle :type Boolean))
  (`/Engine/EditorBlueprintResources/ActorMacros.Switch Has Authority`
    (:`Authority`
      (if (or bForced (not (`KismetMathLibrary.Vector_IsZero` (`self.GetVelocity`))))
        (`KismetSystemLibrary.K2_ClearAndInvalidateTimerHandle` (`self.IdleTimer`))
        (bind _returnvalue (`KismetSystemLibrary.K2_SetTimerDelegate` (`|CreateDelegate` :!event `DetectedByIdle`) (select `bool` bIsIdle :`false` (`self.IdleTimeout`) :`true` (`self.DetectionTime`))))
        (set `self.IdleTimer` _returnvalue)))))

(fn `UpdateDetectedState`
  (params (bForceDetected :type Boolean))
  (bind _weaponmaterial (`self.WeaponMaterial`))
  (bind _returnvalue (or bForceDetected (`self.bIsDetected`)))
  (`|ExecutionSequence`
    (:`then_0`
      (`/Engine/EditorBlueprintResources/StandardMacros.IsValid` _weaponmaterial
        (:`Is Valid`
          (`MaterialInstanceDynamic.SetScalarParameterValue` _weaponmaterial "Painted" (`KismetMathLibrary.Conv_BoolToDouble` _returnvalue)))))
    (:`then_1`
      (`MaterialInstanceDynamic.SetScalarParameterValue` (`self.MaskMaterial`) "Painted" (`KismetMathLibrary.Conv_BoolToDouble` _returnvalue)))))

(fn `UpdateProps`
  (`StaticMeshComponent.SetStaticMesh` (`self.Mask`) (select `int` (select `bool` (`self.bFixedProps`) :`false` (`KismetMathLibrary.RandomIntegerInRange` 0 1) :`true` (`self.MaskID`)) :`0` "/Game/Props/Mask/Mask_01.Mask_01" :`1` "/Game/Props/Mask/Mask_02.Mask_02" :!type "StaticMesh Object Reference"))
  (`StaticMeshComponent.SetStaticMesh` (`self.Weapon`) (select `int` (select `bool` (`self.bFixedProps`) :`false` (`KismetMathLibrary.RandomIntegerInRange` 0 1) :`true` (`self.WeaponID`)) :`0` "/Game/Props/Gun/Patch_1.Patch_1" :`1` "/Game/Props/Gun/Patch_2.Patch_2" :!type "StaticMesh Object Reference")))

(fn `UserConstructionScript`
  (`self.UpdateProps`))