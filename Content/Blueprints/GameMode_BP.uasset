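; Game mode that runs a timed stage progression and notifies VHPlayerController when a player restarts.
; BeginPlay starts a one-shot timer from StageTimeouts, and NextStage increments the stage, re-arms the timer and calls PaintAll on Wall_BP actors tagged "Stage" plus the number.
; When timeouts run out it prints "Game over" and waits, but match exit is unfinished and QuitGame is unconnected.
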(event `self.K2_OnRestartPlayer`
  (params (NewPlayer :type "Controller Object Reference"))
  (bind _asvhplayer_controller (cast `/Game/Blueprints/VHPlayerController` NewPlayer))
  (`/Game/Blueprints/VHPlayerController.OnRespawn` _asvhplayer_controller))

(event `self.ReceiveBeginPlay`
  (`self.ActivateStage`))

(event `NextStage`
  (`/Engine/EditorBlueprintResources/StandardMacros.IncrementInt` (`self.Stage`)
    (:`  `
      (bind _bactivated (`self.ActivateStage`))
      (if _bactivated
        (bind _outactors (`GameplayStatics.GetAllActorsWithTag` (`KismetStringLibrary.Conv_StringToName` (`KismetStringLibrary.Concat_StrStr` "Stage" (`KismetStringLibrary.Conv_IntToString` (`self.Stage`))))))
        (for _array_element _outactors
          (bind _aswall_bp (cast `/Game/Blueprints/Wall_BP` _array_element))
          (`/Game/Blueprints/Wall_BP.PaintAll` _aswall_bp))
        (else
          (`KismetSystemLibrary.PrintString` "Game over")
          (bind _returnvalue (`self.GetNumPlayers`))
          (for _ (range _returnvalue)
            _)
          ;[1 1 1] TODO: exit match ?
          (`KismetSystemLibrary.Delay` 5.0))))))

(fn `ActivateStage`
  (returns (bActivated :type Boolean))
  (`KismetSystemLibrary.K2_ClearAndInvalidateTimerHandle` (`self.StageTimer`))
  (if (`KismetArrayLibrary.Array_IsValidIndex` (`self.StageTimeouts`) (`self.Stage`))
    (bind _returnvalue (`KismetSystemLibrary.K2_SetTimerDelegate` (`|CreateDelegate` :!event `NextStage`) (`|GetArrayItem` (`self.StageTimeouts`) (`self.Stage`))))
    (set `self.StageTimer` _returnvalue)
    (return true)
    (else
      (return false))))

(fn `UserConstructionScript`)