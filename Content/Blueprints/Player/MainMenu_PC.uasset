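; Main menu player controller that shows the menu widget with UI-only input and a visible cursor, and handles LAN matchmaking.
; FindGame searches for LAN sessions and joins the first result.
; If the search fails, it creates a session and opens FirstPersonExampleMap as a listen server.
; A failed join or session creation calls UpdateState on the menu widget, with debug prints logging the outcomes.
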(event `self.ReceiveBeginPlay`
  (bind _returnvalue (`|CreateWidget` "/Game/UI/MainMenu/MainMenu_WBP.MainMenu_WBP_C" self))
  (bind _output_get (set `self.MainMenu` _returnvalue))
  (`UserWidget.AddToViewport` _output_get 0)
  (`WidgetBlueprintLibrary.SetInputMode_UIOnlyEx` self (`self.MainMenu`))
  (set `self.bShowMouseCursor` true))

(event `FindGame`
  (bind _results (`FindSessionsCallbackProxy.FindSessions` self 10 true)
    (:`OnSuccess`
      (`KismetSystemLibrary.PrintString` "MainMenu_PC::FindGame--> Succesfully Found Session" true true (struct :`G` 1.0 :`A` 1.0) 20.0)
      (bind _output (`|GetArrayItem` _results))
      (`JoinSessionCallbackProxy.JoinSession` self _output
        (:`OnSuccess`
          (`KismetSystemLibrary.PrintString` "MainMenu_PC::FindGame--> Succesfully Joined Session" true true (struct :`G` 1.0 :`A` 1.0) 20.0))
        (:`OnFailure`
          (`KismetSystemLibrary.PrintString` (`KismetStringLibrary.Concat_StrStr` "MainMenu_PC::FindGame--> Failed to Join Session (" (`KismetStringLibrary.Conv_IntToString` (`FindSessionsCallbackProxy.GetMaxPlayers` _output)) " )") true true (struct :`R` 1.0 :`G` 1.0 :`A` 1.0) 20.0)
          (`/Game/UI/MainMenu/MainMenu_WBP.UpdateState` (`self.MainMenu`) true))))
    (:`OnFailure`
      (`KismetSystemLibrary.PrintString` "MainMenu_PC::FindGame--> Failed to Find Session" true true (struct :`R` 1.0 :`G` 1.0 :`A` 1.0) 20.0)
      (`CreateSessionCallbackProxy.CreateSession` self 32 true
        (:`OnSuccess`
          (`GameplayStatics.OpenLevel` "FirstPersonExampleMap" true "listen"))
        (:`OnFailure`
          (`KismetSystemLibrary.PrintString` "MainMenu_PC::FindGame--> Failed to Create Session" true true (struct :`R` 1.0 :`A` 1.0) 20.0)
          (`/Game/UI/MainMenu/MainMenu_WBP.UpdateState` (`self.MainMenu`) true))))))

(fn `UserConstructionScript`)