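; VHCharacterMenu_BP is a character Blueprint for the menu that adds a mask render capture to its parent class.
; On BeginPlay it runs the parent logic and sets the detected state to true.
; When props update and a local character is valid, it points MaskCapture2D at Mask_RT and captures the scene once, refreshing the mask render target.
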(event `self.ReceiveBeginPlay`
  (`parent.ReceiveBeginPlay`)
  (`self.UpdateDetectedState` true))

(event `self.UpdateProps`
  (bind _maskcapture2d (`self.MaskCapture2D`))
  (`parent.UpdateProps`)
  (if (`self.bLocalCharacter`)
    (set `SceneCaptureComponent2D.TextureTarget` "/Game/UI/MenuComponents/Mask_RT.Mask_RT" _maskcapture2d)
    (`SceneCaptureComponent2D.CaptureScene` _maskcapture2d)))

(fn `UserConstructionScript`
  (`parent.UserConstructionScript`))