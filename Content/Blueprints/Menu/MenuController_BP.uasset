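; Menu player controller that creates the main menu widget and switches the local player between MainMenu and Lobby states.
; Tick glides the pawn to the state's tagged location and shows or flattens lobby bases through Z scale.
; Paired DoOnce gates alternate transitions: entering Lobby finds and joins a session or creates one, while returning removes remote characters and destroys it.
; A self-restarting timer pulses a scan effect through material parameter collection values.
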(event `self.ReceiveBeginPlay`
  (if (`self.IsLocalPlayerController`)
    (`|ExecutionSequence`
      (:`then_0`
        ;[1 1 1] Find Lobby bases
        (bind _outactors (`GameplayStatics.GetAllActorsWithTag` "LobbyLocations"))
        (set `self.LobbyItems` _outactors))
      (:`then_1`
        ;[1 1 1] Set MainMenu state
        (`self.UpdateMenuState` "NewEnumerator0"))
      (:`then_2`
        ;[1 1 1] Create MainMenu widget
        (bind _returnvalue (`|CreateWidget` "/Game/UI/MainMenu.MainMenu_C" self))
        (bind _output_get (set `self.MenuUI` _returnvalue))
        (`UserWidget.AddToViewport` _output_get 999))
      (:`then_3`
        ;[1 1 1] Launch Scan timer
        (bind _returnvalue_2 (`KismetSystemLibrary.K2_SetTimerDelegate` (delegate `OnScanTimer`) (`self.DemoScanTimeout`) :!label _label))
        (set `self.ScanTimer` _returnvalue_2)))))

(event `SetScanTimer`
  ;[1 1 1] Launch Scan timer
  (goto _label))

(event `OnScanTimer`
  ;[1 1 1] Launch scan effect
  (`KismetSystemLibrary.K2_ClearAndInvalidateTimerHandle` (`self.ScanTimer`))
  (`|ExecutionSequence`
    (:`then_0`
      (`KismetMaterialLibrary.SetVectorParameterValue` "/Game/Materials/ScanParameters.ScanParameters" "Location" (`KismetMathLibrary.Conv_VectorToLinearColor` (`self.K2_GetActorLocation`)))
      (`KismetMaterialLibrary.SetScalarParameterValue` "/Game/Materials/ScanParameters.ScanParameters" "LaunchTime" (`GameplayStatics.GetTimeSeconds`))
      (`KismetMaterialLibrary.SetScalarParameterValue` "/Game/Materials/ScanParameters.ScanParameters" "Power" 1.0))
    (:`then_1`
      (`KismetSystemLibrary.RetriggerableDelay` 5.0)
      (`KismetMaterialLibrary.SetScalarParameterValue` "/Game/Materials/ScanParameters.ScanParameters" "Power")
      (`self.SetScanTimer`))))

(event `TransitionToLobby`
  ;[1 1 1] Transitions between Menu and Lobby
  (if (`self.IsLocalPlayerController`)
    (`/Engine/EditorBlueprintResources/StandardMacros.DoOnce` false :!label _label_2
      (:`Completed`
        (`|ExecutionSequence`
          (:`then_0`
            (goto _label_3 :!via `Reset`))
          (:`then_1`
            (`self.UpdateMenuState` "NewEnumerator1")
            (`self.StartMatchmaking`)))))))

(event `TransitionToMenu`
  ;[1 1 1] Transitions between Menu and Lobby
  (if (`self.IsLocalPlayerController`)
    (`/Engine/EditorBlueprintResources/StandardMacros.DoOnce` true :!label _label_3
      (:`Completed`
        (`|ExecutionSequence`
          (:`then_0`
            (goto _label_2 :!via `Reset`))
          (:`then_1`
            (`|ExecutionSequence`
              (:`then_0`
                (bind _outactors (`GameplayStatics.GetAllActorsWithTag` "RemoteCharacter"))
                (for _array_element _outactors
                  (`self.K2_DestroyActor` _array_element)))
              (:`then_1`
                (`self.CancelLobby`
                  (:`Done`
                    (`self.UpdateMenuState` "NewEnumerator0")))))))))))

(event `self.ReceiveTick`
  (params (DeltaSeconds :type "Float (single-precision)"))
  (if (`self.IsLocalPlayerController`)
    (`|ExecutionSequence`
      (:`then_0`
        (bind _playerpawn (`self.PlayerPawn`)
          (:`then`
            ;[1 1 1] Move camera to Lobby position
            (`self.K2_SetActorLocation` _playerpawn (`KismetMathLibrary.VInterpTo` (`self.K2_GetActorLocation` _playerpawn) (`self.TransitionTarget`) DeltaSeconds (`self.TransitionSpeed`)) false false))
          (:`else`
            ;[1 1 1] Find player's pawn if not already found
            (set `self.PlayerPawn` (`GameplayStatics.GetPlayerPawn` 0)))))
      (:`then_1`
        ;[1 1 1] Hide Lobby bases
        (for _array_element (`self.LobbyItems`)
          (bind (_returnvalue_x _returnvalue_y _returnvalue_z) (`KismetMathLibrary.BreakVector` (`self.GetActorScale3D` _array_element)))
          (`self.SetActorScale3D` _array_element (`KismetMathLibrary.MakeVector` _returnvalue_x _returnvalue_y (select `/Game/UI/MenuComponents/MenuState` (`self.MenuState`) :`NewEnumerator1` 1.0 :!type "Float (single-precision)"))))))))

(event `StartMatchmaking`
  (`KismetSystemLibrary.PrintString` "Find sessions...")
  (bind _results (`FindSessionsCallbackProxy.FindSessions` self 1)
    (:`OnSuccess`
      (if (> (`KismetArrayLibrary.Array_Length` _results) 0)
        (bind _output_get (set `self.CurrentSession` (`|GetArrayItem` _results)))
        (`JoinSessionCallbackProxy.JoinSession` self _output_get
          (:`OnSuccess`
            (`KismetSystemLibrary.PrintString` (`KismetStringLibrary.Concat_StrStr` "Joined, players num: " (`KismetStringLibrary.Conv_IntToString` (`FindSessionsCallbackProxy.GetCurrentPlayers` (`self.CurrentSession`))))))
          (:`OnFailure`
            (`KismetSystemLibrary.PrintString` "Can't join sessions")))
        (else
          (`KismetSystemLibrary.PrintString` "Can't find sessions" :!label _label_4)
          (`CreateSessionCallbackProxy.CreateSession` self 5
            (:`OnSuccess`
              (`KismetSystemLibrary.PrintString` "Session created"))
            (:`OnFailure`
              (`self.TransitionToMenu`)
              (`KismetSystemLibrary.PrintString` "Can't create session!"))))))
    (:`OnFailure`
      (`KismetSystemLibrary.PrintString` "FindSessions failed")
      (goto _label_4))))

(event `ExitGame`
  (`self.CancelLobby`
    (:`Done`
      (`KismetSystemLibrary.QuitGame` null "Quit"))))

(fn `UpdateMenuState`
  (params (MenuState :type "/Game/UI/MenuComponents/MenuState Enum" :default "NewEnumerator0"))
  (bind _output_get (set `self.MenuState` MenuState))
  (`|ExecutionSequence`
    (:`then_0`
      (bind _outactors (`GameplayStatics.GetAllActorsWithTag` (select `/Game/UI/MenuComponents/MenuState` _output_get :`NewEnumerator0` "StartLocation" :`NewEnumerator1` "LobbyLocation" :!type "Name")))
      (set `self.TransitionTarget` (`self.K2_GetActorLocation` (`|GetArrayItem` _outactors))))
    (:`then_1`
      (bind _menuui (`self.MenuUI`)
        (:`then`
          (`/Game/UI/MainMenu.UpdateMenuState` _menuui (`self.MenuState`)))
        (:`else`)))))

(fn `UserConstructionScript`)