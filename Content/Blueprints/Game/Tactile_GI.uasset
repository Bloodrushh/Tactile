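; Game instance Blueprint that handles quick LAN matchmaking from the main menu through a FindGame event.
; It clears the menu's server rows, searches for LAN sessions and joins the first one found.
; If none is found or the search fails, it creates a session and opens the first-person example map as a listen server.
; A failed join lists that session in the menu, and failed joins or creations update the menu state.
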(event `FindGame`
  (bind _asmain_menu_pc (cast `/Game/Blueprints/Player/MainMenu_PC` (`GameplayStatics.GetPlayerController` 0)))
  (set `self.MainMenu` (`/Game/Blueprints/Player/MainMenu_PC.MainMenu` _asmain_menu_pc))
  (`/Game/UI/MainMenu/MainMenu_WBP.ClearServerRows` (`self.MainMenu`))
  (bind _results (`FindSessionsCallbackProxy.FindSessions` (`GameplayStatics.GetPlayerController` 0) 1000 true)
    (:`OnSuccess`
      (bind _output_get (set `self.FoundSessions` _results))
      (if (> (`KismetArrayLibrary.Array_Length` _output_get) 0)
        (`KismetSystemLibrary.PrintString` "MainMenu_PC::FindGame--> Succesfully Found Session" true true (struct :`G` 1.0 :`A` 1.0) 20.0)
        (`JoinSessionCallbackProxy.JoinSession` (`GameplayStatics.GetPlayerController` 0) (`|GetArrayItem` (`self.FoundSessions`))
          (:`OnSuccess`
            (`KismetSystemLibrary.PrintString` "MainMenu_PC::FindGame--> Succesfully Joined Session" true true (struct :`G` 1.0 :`A` 1.0) 20.0))
          (:`OnFailure`
            (`KismetSystemLibrary.PrintString` "MainMenu_PC::FindGame--> Failed to Join Session" true true (struct :`R` 1.0 :`G` 1.0 :`A` 1.0) 20.0)
            (`/Game/UI/MainMenu/MainMenu_WBP.AddServerRow` (`self.MainMenu`) (`|GetArrayItem` (`self.FoundSessions`)))
            (`/Game/UI/MainMenu/MainMenu_WBP.UpdateState` (`self.MainMenu`) true)))
        (else
          (`KismetSystemLibrary.PrintString` "MainMenu_PC::FindGame--> Failed to Find Session" true true (struct :`R` 1.0 :`G` 1.0 :`A` 1.0) 20.0 :!label _label)
          (`CreateSessionCallbackProxy.CreateSession` (`GameplayStatics.GetPlayerController` 0) 4 true
            (:`OnSuccess`
              (`GameplayStatics.OpenLevel` "FirstPersonExampleMap" true "listen"))
            (:`OnFailure`
              (`KismetSystemLibrary.PrintString` "MainMenu_PC::FindGame--> Failed to Create Session" true true (struct :`R` 1.0 :`A` 1.0) 20.0)
              (`/Game/UI/MainMenu/MainMenu_WBP.UpdateState` (`self.MainMenu`) true))))))
    (:`OnFailure`
      (goto _label))))