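; VHPlayerController is a player controller that manages the gameplay HUD and handles player death and respawn.
; On the local controller, BeginPlay creates the GameplayUI widget and adds it to the viewport.
; Death, intended for the server, destroys the controlled pawn and restarts the player through the game mode.
; OnRespawn, called client-side by the newly possessed pawn, tells the UI to update its owner.
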(event `self.ReceiveBeginPlay`
  ;[1 1 1] [Client] Create UI
  (if (`self.IsLocalController`)
    (bind _returnvalue (`|CreateWidget` "/Game/UI/GameplayUI.GameplayUI_C" self))
    (bind _output_get (set `self.UI` _returnvalue))
    (`UserWidget.AddToViewport` _output_get 0)))

(event `Death`
  ;[1 1 1] [Server] On death happened
  (`self.K2_DestroyActor` (`self.K2_GetPawn`))
  (`GameModeBase.RestartPlayer` (`GameplayStatics.GetGameMode`) self))

(event `OnRespawn`
  ;[1 1 1] [Client] Update UI after respawn;
  ; Called from the possessed pawn on the client side when it's possessed
  (bind _ui (`self.UI`)
    (:`then`
      (`/Game/UI/GameplayUI.UpdateOwner` _ui))
    (:`else`)))

(fn `UserConstructionScript`)