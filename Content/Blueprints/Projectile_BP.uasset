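; Projectile actor that detects hits on characters and world geometry on the server, then damages the character hit.
; Character overlaps trigger short component line traces along the velocity, testing the hair mesh before the body mesh for precise collision.
; Both trace and blocking hits feed MarkHitPoint, which draws a debug-point paint splash, deactivates, applies the shooter's Damage to character targets and destroys the projectile.
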(event `self.ReceiveActorBeginOverlap`
  (params (OtherActor :type "Actor Object Reference"))
  ;[1 1 1] [Server] Check complex collision against the CHaracter meshes
  (`/Engine/EditorBlueprintResources/ActorMacros.Switch Has Authority`
    (:`Authority`
      (bind _asvhcharacter_bp (cast `/Game/Blueprints/VHCharacter_BP` OtherActor))
      ;;[1 1 1] Trace for Hair first, if no collision then trace for mesh
      (bind _returnvalue (`self.TraceAgainstComponent` (`/Game/Blueprints/VHCharacter_BP.Hair_Mesh` _asvhcharacter_bp)))
      (if (not _returnvalue)
        (`self.TraceAgainstComponent` (`Character.Mesh` _asvhcharacter_bp))))))

(event `self.ReceiveHit`
  (params (MyComp :type "PrimitiveComponent Object Reference") (Other :type "Actor Object Reference") (OtherComp :type "PrimitiveComponent Object Reference") (bSelfMoved :type Boolean) (HitLocation :type "Vector Structure") (HitNormal :type "Vector Structure") (NormalImpulse :type "Vector Structure") (Hit :type "HitResult Structure (by ref)"))
  ;[1 1 1] [Server] hit world static
  (`/Engine/EditorBlueprintResources/ActorMacros.Switch Has Authority`
    (:`Authority`
      (`self.MarkHitPoint` HitLocation))))

(event `MarkHitPoint`
  (params (Position :type "Vector Structure") (HitActor :type "Actor Object Reference"))
  ;[1 1 1] [Server] Projectile hits something
  (if (and (`self.HasAuthority`) (`self.bActive`))
    (`|ExecutionSequence`
      (:`then_0`
        (`self.OnTargetPaint` Position))
      (:`then_1`
        (set `self.bActive` false))
      (:`then_2`
        (bind _asvoid_hunters_character (cast `VoidHuntersCharacter` HitActor))
        (bind _asvoid_hunters_character_2 (cast `VoidHuntersCharacter` (`self.GetShooter`)))
        (`GameplayStatics.ApplyDamage` _asvoid_hunters_character (`VoidHuntersCharacter.Damage` _asvoid_hunters_character_2) (`Pawn.GetController` _asvoid_hunters_character_2) self "/Script/Engine.DamageType"))
      (:`then_3`
        (`self.K2_DestroyActor`)))))

(event `OnTargetPaint`
  (params (Position :type "Vector Structure"))
  ;[1 1 1] [Client] Draw paint splash
  (`KismetSystemLibrary.DrawDebugPoint` Position 10.0 (struct :`R` 0.994792 :`G` 0.989583 :`B` 1.0 :`A` 1.0) 10.0))

(fn `TraceAgainstComponent`
  (params (Component :type "PrimitiveComponent Object Reference"))
  (returns (ReturnValue :type Boolean))
  (bind _returnvalue (`self.K2_GetActorLocation`))
  (bind (_hitlocation _hitnormal _bonename _outhit _returnvalue_2) (`PrimitiveComponent.K2_LineTraceComponent` Component _returnvalue (+ _returnvalue (* (`KismetMathLibrary.Normal` (`MovementComponent.Velocity` (`self.ProjectileMovement`))) 50.0)) true false false))
  (if _returnvalue_2
    (`self.MarkHitPoint` _hitlocation (`ActorComponent.GetOwner` Component)))
  (return _returnvalue_2))

(fn `UserConstructionScript`)